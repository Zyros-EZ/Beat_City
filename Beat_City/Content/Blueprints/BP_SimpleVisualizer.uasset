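; BP_SimpleVisualizer is an audio analysis debug actor that plays a sound and prints its analysis on screen during playback.
; The playback-percent callback converts progress to seconds and samples Constant-Q and loudness NRT assets at that time.
; It prints Constant-Q values alongside cooked FFT magnitudes at preset frequencies.
; Loudness updates running min/max values and increments a crude beat count whenever it falls within a fixed range.
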(event `self.ReceiveBeginPlay`
  (`AudioComponent.SetSound` (`self.Audio`) (`self.New Sound`))
  (set `self.Duration` (`SoundBase.Duration` (`self.New Sound`)))
  (add `AudioComponent.OnAudioPlaybackPercent` (`self.Audio`) (delegate `Playback Audio Percent`))
  (`AudioComponent.Play` (`self.Audio`) 0.0))

(event `Playback Audio Percent`
  (params (PlayingSoundWave :type "SoundWave Object Reference") (PlaybackPercent :type "Float (single-precision)"))
  (bind _returnvalue (* PlaybackPercent (`self.Duration`)))
  (bind _outloudness (`LoudnessNRT.GetLoudnessAtTime` (`self.LoudnessNRT Ref`) _returnvalue))
  (`|ExecutionSequence`
    (:`then_0`
      (bind _output_get (set `self.Played Time` _returnvalue))
      (for _array_element (`ConstantQNRT.GetNormalizedChannelConstantQAtTime` (`self.Constant NRT Ref`) _output_get 0)
        (`KismetSystemLibrary.PrintString` (`KismetStringLibrary.Conv_DoubleToString` _array_element) true true (struct :`G` 0.66 :`B` 1.0 :`A` 1.0) 0.0 (`self.Key`))
        (bind _outsoundwavespectraldata (`AudioComponent.GetCookedFFTData` (`self.Audio`) (`|MakeArray` 100.0 500.0 1000.0 5000.0 :!type "Float (single-precision)")))
        (`KismetSystemLibrary.PrintString` (`KismetStringLibrary.Concat_StrStr` (`KismetStringLibrary.Conv_DoubleToString` (`.Magnitude` (break `SoundWaveSpectralData` (`|GetArrayItem` _outsoundwavespectraldata)))) ", " (`KismetStringLibrary.Conv_DoubleToString` (`.Magnitude` (break `SoundWaveSpectralData` (`|GetArrayItem` _outsoundwavespectraldata 1)))) ", " (`KismetStringLibrary.Conv_DoubleToString` (`.Magnitude` (break `SoundWaveSpectralData` (`|GetArrayItem` _outsoundwavespectraldata 2)))) ", " (`KismetStringLibrary.Conv_DoubleToString` (`.Magnitude` (break `SoundWaveSpectralData` (`|GetArrayItem` _outsoundwavespectraldata))))) true true (struct :`G` 0.66 :`B` 1.0 :`A` 1.0) 2.0 (`self.Key_0`))))
    (:`then_1`
      (`self.Get Min max Value` _outloudness)
      (`KismetSystemLibrary.PrintString` (`KismetStringLibrary.Concat_StrStr` "Loudness: " "Min: " (`KismetStringLibrary.Conv_DoubleToString` (`self.Min Loud Value`)) ", " "Max: " (`KismetStringLibrary.Conv_DoubleToString` (`self.Max Loud Value`)) ", " (`KismetStringLibrary.Conv_DoubleToString` _outloudness) ", " "Beats: " (`KismetStringLibrary.Conv_DoubleToString` (`self.Beat Count`))) true true (struct :`G` 0.66 :`B` 1.0 :`A` 1.0) 15.0 (`self.Loudness`)))))

(event `self.ReceiveTick`
  (params (DeltaSeconds :type "Float (single-precision)")))

(fn `Get Min max Value`
  (params (`In Value` :type "Float (double-precision)"))
  (`|ExecutionSequence`
    (:`then_0`
      (if (< `In Value` (`self.Min Loud Value`))
        (set `self.Min Loud Value` `In Value`)))
    (:`then_1`
      (if (> `In Value` (`self.Max Loud Value`))
        (set `self.Max Loud Value` `In Value`)))
    (:`then_2`
      (if (`KismetMathLibrary.InRange_FloatFloat` `In Value` -30.0 -24.0)
        (`/Engine/EditorBlueprintResources/StandardMacros.IncrementFloat` (`self.Beat Count`))))))

(fn `UserConstructionScript`)