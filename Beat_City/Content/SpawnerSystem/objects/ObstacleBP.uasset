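; Spawner-system obstacle that takes a random prop mesh (trashcan, plant, barrel, box or barricade) in its construction script and can damage the player.
; TopRow, MidRow and bottomrow events play timelines that set its transform from the matching ControlSpawn spline, using spline direction as location.
; On overlapping the player, it deals damage once and destroys itself if IsDangerus is set.
; Music-note mesh selection and the spawner lookup sit in unconnected logic.
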(event `Determine`
  ;[1 0.1419 0.6154 1 36] Determines what to spawn - random chance to spawn a damage dealing object
  (switch `int` (`KismetMathLibrary.RandomIntegerInRange` 0 4)
    (:`0`
      (set `self.type` "NewEnumerator0"))
    (:`1`
      (set `self.type` "NewEnumerator1"))
    (:`2`
      (set `self.type` "NewEnumerator2"))
    (:`3`
      (set `self.type` "NewEnumerator3"))
    (:`4`
      (set `self.type` "NewEnumerator6")))
  (`self.model`))

(event `self.ReceiveBeginPlay`
  ;[0.07005 0.3588 1 1 30] when spawned -> set type variable -> goes to change model
  (bind _asbp_player_character (cast `/Game/ThirdPerson/Blueprints/Characters/BP_Player_Character` (`GameplayStatics.GetPlayerPawn` 0)))
  (set `self.Player` _asbp_player_character))

(event `Top Row`
  (bind _top (`/Game/SpawnerSystem/objects/spawner.top` (`self.control spawn`)))
  ;[0.04585 1 0.02567 1 36] Sets movement speed -> looks for the spline -> Moves across it
  (bind _output_get (set `self.movement` 5.0))
  (`TimelineComponent.SetPlayRate` (`self.T Rythm`) (/ 1.0 _output_get))
  (bind (_direction _newtrack_0) (`Timeline|T Rythm` :!via `PlayFromStart`)
    (:`Update`
      (bind _returnvalue (`KismetMathLibrary.Lerp` 0.0 (`SplineComponent.GetSplineLength` _top) _newtrack_0))
      (`self.K2_SetActorTransform` (`KismetMathLibrary.MakeTransform` (`SplineComponent.GetDirectionAtDistanceAlongSpline` _top _returnvalue "Local") (`SplineComponent.GetRotationAtDistanceAlongSpline` _top _returnvalue "Local") (`SceneComponent.RelativeScale3D` (`self.body`)))))))

(event `self. damagezone.OnComponentBeginOverlap`
  (params (OverlappedComponent :type "PrimitiveComponent Object Reference") (OtherActor :type "Actor Object Reference") (OtherComp :type "PrimitiveComponent Object Reference") (OtherBodyIndex :type Integer) (bFromSweep :type Boolean) (SweepResult :type "HitResult Structure (by ref)"))
  ;[1 0.009947 0 1 36] If overlapping player -> Checks if its not a note -> if Yes -> Deal Damage -> despawn
  (if (`PrimitiveComponent.IsOverlappingActor` OverlappedComponent (`self.Player`))
    (if (`self.is dangerus`)
      (`/Engine/EditorBlueprintResources/StandardMacros.DoOnce` false
        (:`Completed`
          (`/Game/ThirdPerson/Blueprints/Characters/BP_Player_Character.Decrease Health` (`self.Player`) 3.0)
          (`self.K2_DestroyActor`))))))

(event `Mid Row`
  (bind _middle (`/Game/SpawnerSystem/objects/spawner.middle` (`self.control spawn`)))
  ;[0.04585 1 0.02567 1 36] Sets movement speed -> looks for the spline -> Moves across it
  (bind _output_get (set `self.movement` 5.0))
  (`TimelineComponent.SetPlayRate` (`self.M Rythm`) (/ 1.0 _output_get))
  (bind (_direction _newtrack_0) (`Timeline|M Rythm` :!via `PlayFromStart`)
    (:`Update`
      (bind _returnvalue (`KismetMathLibrary.Lerp` 0.0 (`SplineComponent.GetSplineLength` _middle) _newtrack_0))
      (`self.K2_SetActorTransform` (`KismetMathLibrary.MakeTransform` (`SplineComponent.GetDirectionAtDistanceAlongSpline` _middle _returnvalue "Local") (`SplineComponent.GetRotationAtDistanceAlongSpline` _middle _returnvalue "Local") (`SceneComponent.RelativeScale3D` (`self.body`)))))))

(event `model`
  (bind _body (`self.body`))
  (bind _body_2 (`self.body`))
  ;[0 1 0.3061 1 30] check type variable -> change body of damaging object
  (switch `/Game/SpawnerSystem/objects/types` (`self.type`)
    (:`NewEnumerator0`
      (`StaticMeshComponent.SetStaticMesh` _body "/Game/SpawnerSystem/objects/assets/TRASH_CAN.TRASH_CAN"))
    (:`NewEnumerator1`
      (`StaticMeshComponent.SetStaticMesh` _body "/Game/SpawnerSystem/objects/assets/PLANT_OUTDOOR.PLANT_OUTDOOR"))
    (:`NewEnumerator2`
      (`StaticMeshComponent.SetStaticMesh` _body_2 "/Game/SpawnerSystem/objects/assets/barrel.barrel"))
    (:`NewEnumerator3`
      (`StaticMeshComponent.SetStaticMesh` _body_2 "/Game/SpawnerSystem/objects/assets/box.box"))
    (:`NewEnumerator6`
      (`StaticMeshComponent.SetStaticMesh` _body_2 "/Game/SpawnerSystem/objects/assets/BARRICADE.BARRICADE"))))

(event `bottom row`
  (bind _bottom (`/Game/SpawnerSystem/objects/spawner.bottom` (`self.control spawn`)))
  ;[0.04585 1 0.02567 1 36] Sets movement speed -> looks for the spline -> Moves across it
  (bind _output_get (set `self.movement` 5.0))
  (`TimelineComponent.SetPlayRate` (`self.B Rythm`) (/ 1.0 _output_get))
  (bind (_direction _newtrack_0) (`Timeline|B Rythm` :!via `PlayFromStart`)
    (:`Update`
      (bind _returnvalue (`KismetMathLibrary.Lerp` 0.0 (`SplineComponent.GetSplineLength` _bottom) _newtrack_0))
      (`self.K2_SetActorTransform` (`KismetMathLibrary.MakeTransform` (`SplineComponent.GetDirectionAtDistanceAlongSpline` _bottom _returnvalue "Local") (`SplineComponent.GetRotationAtDistanceAlongSpline` _bottom _returnvalue "Local") (`SceneComponent.RelativeScale3D` (`self.body`)))))))

(fn `UserConstructionScript`
  (`self.Determine`))